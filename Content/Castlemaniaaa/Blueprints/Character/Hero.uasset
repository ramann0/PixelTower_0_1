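; Player hero Blueprint for a side-scrolling character with movement, jumping and a ranged arrow attack.
; Input drives the pixel movement component, flips control yaw to face left or right, and maintains moving, jumping and falling flags.
; E starts the attack state; a projectile-release event fires arrows through BPAttackComponent, then reopens the DoOnce gate after an AttackSpeed delay.
; BeginPlay sets the view target to CharCamera's owner.
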(event `RangedAnimationFinished`
  (set `self.bIsRangedAttacking` false))

(event `Key|E`
  (params (Key :type "Key Structure"))
  (:`Pressed`
    (if (not (`self.bIsRangedAttacking`))
      (`/Engine/EditorBlueprintResources/StandardMacros.DoOnce` false :!label _label
        (:`Completed`
          (set `self.bIsRangedAttacking` true))))))

(event `RangedProjectileReleased`
  (`/Game/Pixel2D/Blueprints/Components/BP_AttackComponent.RangedAttack` :`self` (`self.BP_AttackComponent`) :`Damage` (`self.damage`) :`SpawnLocation` (`SceneComponent.K2_GetComponentLocation` (`self.Arrow1`)) :`ProjectileSpeed` (`self.projectileSpeed`) :`ProjectilesSpawned` (`self.projectileSpawned`) :`TimeBetweenProjectiles` (`self.timeBetweenProjectiles`) :`AttackSpeed` (`self.attackSpeed`) :`ProjectileActorClass` "/Game/Castlemaniaaa/Blueprints/Character/BetterMegaArrow.BetterMegaArrow_C" :`Direction` (`self.GetActorForwardVector`) :`ProjectileTravelDistance` 100.0 :`CollidesWithWorld?` true :`KnockbackForce` (`self.knockbackForce`))
  (`KismetSystemLibrary.Delay` (`self.attackSpeed`))
  (goto _label :!via `Reset`))

(event `Key|Q`
  (params (Key :type "Key Structure")))

(event `self.OnWalkingOffLedge`
  (params (PreviousFloorImpactNormal :type "Vector Structure (by ref)") (PreviousFloorContactNormal :type "Vector Structure (by ref)") (PreviousLocation :type "Vector Structure (by ref)") (TimeDelta :type "Float (single-precision)"))
  (set `self.bIsFalling` true)
  (set `self.bIsMoving` false)
  (set `self.bIsJumping` false))

(event `self.OnLanded`
  (params (Hit :type "HitResult Structure (by ref)"))
  (set `self.bIsFalling` false)
  (set `self.bIsJumping` false))

(event `InputAction|Jump`
  (params (Key :type "Key Structure"))
  (bind _bp_pixelcharactermovementcomponent (`self.BP_PixelCharacterMovementComponent`))
  (:`Pressed`
    (bind _canjump_ (`/Game/Pixel2D/Blueprints/Components/BP_PixelCharacterMovementComponent.Jump` _bp_pixelcharactermovementcomponent 0.0))
    (if _canjump_
      (set `self.bIsJumping` true)
      (`KismetSystemLibrary.Delay` 0.1)
      (set `self.bIsJumping` false)
      (set `self.bIsFalling` true)))
  (:`Released`
    (`/Game/Pixel2D/Blueprints/Components/BP_PixelCharacterMovementComponent.EndJumping` _bp_pixelcharactermovementcomponent)))

(event `InputAxis|MoveRight`
  (params (AxisValue :type "Float (single-precision)"))
  (bind _returnvalue (`self.GetController`))
  (bind _ismoving (`/Game/Pixel2D/Blueprints/Components/BP_PixelCharacterMovementComponent.Move` (`self.BP_PixelCharacterMovementComponent`) (`GameplayStatics.GetPlayerPawn` 0) AxisValue))
  (set `self.bIsMoving` _ismoving)
  (`/Engine/EditorBlueprintResources/StandardMacros.CompareFloat` AxisValue
    (:`>`
      (`Controller.SetControlRotation` _returnvalue (`KismetMathLibrary.MakeRotator` 0.0)))
    (:`<`
      (`Controller.SetControlRotation` _returnvalue (`KismetMathLibrary.MakeRotator` 0.0 0.0 180.0)))))

(event `self.ReceiveBeginPlay`
  (`PlayerController.SetViewTargetWithBlend` (`GameplayStatics.GetPlayerController` 0) (`ActorComponent.GetOwner` (`self.Char_Camera`)) 0.0 "VTBlend_Linear" 0.0 false))

(fn `UserConstructionScript`)